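; Ballista turret structure that supports default, explosive and tranquilizer arrows.
; It matches the class display name of the first inventory item to pick the projectile class, and also the ammo item template for explosive and tranq arrows.
; The same check swaps the material on the skeletal mesh to show the arrow type.
; A separate reset function restores the ammo template to the reload ammo type.
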(fn `Reset for Reload`
  (set `self.AmmoItemTemplate` (`self.ReloadAmmoType`)))

(fn `Set Ammo Explosive`
  (set `self.ProjectileClass` "/Game/Mods/GREKT/Ballista/ProjBallistaExplosive.ProjBallistaExplosive_C")
  (set `self.AmmoItemTemplate` "/Game/Mods/GREKT/Ballista/PrimalItemAmmo_BallistaArrow_Explosive.PrimalItemAmmo_BallistaArrow_Explosive_C"))

(fn `Set Ammo Tranq`
  (set `self.ProjectileClass` "/Game/Mods/GREKT/Ballista/ProjBallistaTranq.ProjBallistaTranq_C")
  (set `self.AmmoItemTemplate` "/Game/Mods/GREKT/Ballista/PrimalItemAmmo_BallistaArrow_Tranq.PrimalItemAmmo_BallistaArrow_Tranq_C"))

(fn `Set Current Ammo`
  (switch `string` (`KismetSystemLibrary.GetClassDisplayName` (`GameplayStatics.GetObjectClass` (`KismetArrayLibrary.Array_Get` (`PrimalInventoryComponent.InventoryItems` (`self.PrimalInventoryBP_Ballista_C1`)))))
    (:`Default`
      (`self.SetAmmo_Default`))
    (:`PrimalItemAmmo_BallistaArrow_Explosive_C`
      (`self.Set Ammo Explosive`))
    (:`PrimalItemAmmo_BallistaArrow_Tranq_C`
      (`self.Set Ammo Tranq`))))

(fn `SetAmmo_Default`
  (set `self.ProjectileClass` "/Game/PrimalEarth/CoreBlueprints/Projectiles/ProjBallista.ProjBallista_C"))

(fn `SetProjectileMesh`
  (bind _skeletalmesh1 (`self.SkeletalMesh1`))
  (switch `string` (`KismetSystemLibrary.GetClassDisplayName` (`GameplayStatics.GetObjectClass` (`KismetArrayLibrary.Array_Get` (`PrimalInventoryComponent.InventoryItems` (`self.PrimalInventoryBP_Ballista_C1`)))))
    (:`Default`
      (`PrimitiveComponent.SetMaterial` _skeletalmesh1 0 "/Game/PrimalEarth/WeaponMountedTurret/Mounted_turret_arrow_MIC.Mounted_turret_arrow_MIC"))
    (:`PrimalItemAmmo_BallistaArrow_Explosive_C`
      (`PrimitiveComponent.SetMaterial` _skeletalmesh1 0 "/Game/Mods/GREKT/Ballista/Mounted_turret_arrow_Explosive_MIC.Mounted_turret_arrow_Explosive_MIC"))
    (:`PrimalItemAmmo_BallistaArrow_Tranq_C`
      (`PrimitiveComponent.SetMaterial` _skeletalmesh1 0 "/Game/Mods/GREKT/Ballista/Mounted_turret_arrow_Tranq_MIC.Mounted_turret_arrow_Tranq_MIC"))))

(fn `UserConstructionScript`)